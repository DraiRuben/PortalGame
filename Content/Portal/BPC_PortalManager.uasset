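; Portal manager component that lets the player place a linked blue and orange portal pair on surfaces.
; The place-portal input fires a Visibility line trace, with the action value's sign choosing the color, and builds a transform from the hit location and normal.
; CreatePortal destroys any existing portal of that color, then spawns and stores a BP_Portal, passing it the hit surface and opposite portal.
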(event `EnhancedInput|/Game/Input/InputActions/IA_PlacePortal`
  (params (ActionValue :type "Float (double-precision)") (ElapsedSeconds :type "Float (double-precision)") (TriggeredSeconds :type "Float (double-precision)") (InputAction :type "InputAction Object Reference" :default "/Game/Input/InputActions/IA_PlacePortal.IA_PlacePortal"))
  (bind (_trace_start _trace_end) (`/Game/Systems/BPFL_FunctionLibrary.Get Trace`))
  (:`Started`
    (bind (_outhit _returnvalue) (`KismetSystemLibrary.LineTraceSingle` _trace_start _trace_end "TraceTypeQuery1"))
    (if _returnvalue
      (if (> ActionValue 0.0)
        (bind (_bblockinghit _binitialoverlap _time _distance _location _impactpoint _normal _impactnormal _physmat _hitactor _hitcomponent) (`GameplayStatics.BreakHitResult` _outhit))
        (bind _transform (`/Game/Systems/BPFL_FunctionLibrary.Make Portal Transform` _location _normal))
        (`self.Create Portal` "NewEnumerator1" _transform _hitcomponent)
        (else
          (`self.Create Portal` "NewEnumerator0" _transform _hitcomponent))))))

(fn `Create Portal`
  (params (`Portal Type` :type "/Game/Portal/EPortalType Enum" :default "NewEnumerator0") (`Portal Transform` :type "Transform Structure") (`Hit Surface` :type "PrimitiveComponent Object Reference"))
  (locals (`Connected Portal` :type "/Game/Portal/BP_Portal Object Reference"))
  (switch `/Game/Portal/EPortalType` `Portal Type`
    (:`NewEnumerator0`
      (`/Engine/EditorBlueprintResources/StandardMacros.IsValid` (`self.OrangePortal`)
        (:`Is Valid`
          (`/Game/Portal/BP_Portal.Destroy Portal` (`self.OrangePortal`)))
        (:`Is Not Valid`
          _))
      (bind _returnvalue (`|SpawnActorFromClass` "/Game/Portal/BP_Portal.BP_Portal_C" `Portal Transform` "Undefined" "MultiplyWithRoot" null (`self.BluePortal`) `Portal Type` `Hit Surface` null))
      (set `self.OrangePortal` _returnvalue))
    (:`NewEnumerator1`
      (`/Engine/EditorBlueprintResources/StandardMacros.IsValid` (`self.BluePortal`)
        (:`Is Valid`
          (`/Game/Portal/BP_Portal.Destroy Portal` (`self.BluePortal`)))
        (:`Is Not Valid`
          _))
      (bind _returnvalue_2 (`|SpawnActorFromClass` "/Game/Portal/BP_Portal.BP_Portal_C" `Portal Transform` "Undefined" "MultiplyWithRoot" null (`self.OrangePortal`) `Portal Type` `Hit Surface` null))
      (set `self.BluePortal` _returnvalue_2))))