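; BP_LaserEmitter is an interactable object that acts as the origin of a laser.
; On BeginPlay it spawns a BP_Laser at its Arrow component's location, using the actor's rotation.
; It passes itself as the emitter and its display name as the laser ID, then adds the new laser to its ChildLasers collection.
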(event `self.ReceiveBeginPlay`
  (set `self.LaserEmitter` self)
  (set `self.ID` (`KismetSystemLibrary.GetDisplayName` self))
  (bind _returnvalue (`|SpawnActorFromClass` "/Game/Interactable/Objects/Laser/BP_Laser.BP_Laser_C" (`KismetMathLibrary.MakeTransform` (`SceneComponent.K2_GetComponentLocation` (`self.Arrow`)) (`self.K2_GetActorRotation`)) "Undefined" "MultiplyWithRoot" null (`self.ID`) (`self.LaserEmitter`) null))
  (`KismetArrayLibrary.Array_Add` (`self.Child Lasers`) _returnvalue))

(fn `UserConstructionScript`
  (`parent.UserConstructionScript`))