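; BP_LaserReceiver is a laser target that triggers a linked ToActivate object.
; LaserBounce sends that object an Interact message, passing itself on a hit and no argument otherwise.
; An older DoOnce path with a ResetDoOnce event remains, but its ConnectedLaser validity check is unreachable and Tick is empty.
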(event `self.ReceiveTick`
  (params (DeltaSeconds :type "Float (single-precision)")))

(event `ResetDoOnce`
  (`/Engine/EditorBlueprintResources/StandardMacros.DoOnce` true :!via `Reset`
    (:`Completed`
      (message `/Game/Interactable/BPI_Interactable.Interact` (`self.ToActivate`) self))))

(fn `LaserBounce`
  (params (HitLaser :type "/Game/Interactable/Objects/Laser/BP_Laser Object Reference") (Hit :type Boolean) (HitInfo :type "HitResult Structure"))
  (returns (NewLaser :type "/Game/Interactable/Objects/Laser/BP_Laser Object Reference"))
  (if Hit
    (message `/Game/Interactable/BPI_Interactable.Interact` (`self.ToActivate`) self)
    (else
      (message `/Game/Interactable/BPI_Interactable.Interact` (`self.ToActivate`) null)))
  (return null))

(fn `UserConstructionScript`
  (`parent.UserConstructionScript`))