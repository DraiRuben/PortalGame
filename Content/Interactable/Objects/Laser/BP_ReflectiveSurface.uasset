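; BP_ReflectiveSurface is an interactable surface that bounces lasers by spawning a new BP_Laser at the impact point.
; LaserBounce orients the new laser along a reflection computed from trace start and hit normal, passing on an updated ID and the same emitter.
; The new laser is registered in both the surface's attached lasers and the emitter's child lasers.
; Without a hit, it clears attached lasers using the incoming laser's ID.
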(event `self.ReceiveBeginPlay`)

(fn `LaserBounce`
  (params (HitLaser :type "/Game/Interactable/Objects/Laser/BP_Laser Object Reference") (Hit :type Boolean) (HitInfo :type "HitResult Structure"))
  (returns (NewLaser :type "/Game/Interactable/Objects/Laser/BP_Laser Object Reference"))
  (bind _hitlaser (`local.HitLaser`))
  (bind (_bblockinghit _binitialoverlap _time _distance _location _impactpoint _normal _impactnormal _physmat _hitactor _hitcomponent _hitbonename _bonename _hititem _elementindex _faceindex _tracestart) (`GameplayStatics.BreakHitResult` (`local.HitInfo`)))
  (if Hit
    (bind _returnvalue (`|SpawnActorFromClass` :`Class` "/Game/Interactable/Objects/Laser/BP_Laser.BP_Laser_C" :`SpawnTransform` (`KismetMathLibrary.MakeTransform` _impactpoint (`/Game/Systems/BPFL_FunctionLibrary.CalculateRelectionRotation` _impactpoint _impactnormal _tracestart)) :`CollisionHandlingOverride` "Undefined" :`TransformScaleMethod` "MultiplyWithRoot" :`LaserID` (`/Game/Interactable/Objects/Laser/BP_Laser.UpdateID` _hitlaser "B") :`LaserEmitter` (`/Game/Interactable/Objects/Laser/BP_LaserParent.LaserEmitter` _hitlaser) :`Instigator` null))
    (`KismetArrayLibrary.Array_Add` (`self.LasersAttached`) _returnvalue)
    (`KismetArrayLibrary.Array_Add` (`/Game/Interactable/Objects/Laser/BP_LaserEmitter.Child Lasers` (`/Game/Interactable/Objects/Laser/BP_LaserParent.LaserEmitter` (`local.HitLaser`))) _returnvalue)
    (return _returnvalue)
    (else
      (`self.ClearAttachedLasers` (`/Game/Interactable/Objects/Laser/BP_Laser.LaserID` (`local.HitLaser`)))
      (return null))))

(fn `UserConstructionScript`)