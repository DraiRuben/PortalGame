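; Base Blueprint for laser objects that tracks laser actors in a LasersAttached array and provides cleanup functions for them.
; ClearAllAttachedLasers destroys every valid attached laser and empties the array.
; ClearAttachedLasers removes only lasers whose LaserID contains the given ID as a substring, looping in reverse so removal during iteration is safe.
; The event graph and construction script are empty, so the class runs no logic by itself.
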(fn `ClearAllAttachedLasers`
  (bind _lasersattached (`self.LasersAttached`))
  (for _array_element _lasersattached
    (`/Engine/EditorBlueprintResources/StandardMacros.IsValid` _array_element
      (:`Is Valid`
        (`self.K2_DestroyActor` _array_element))))
  (`KismetArrayLibrary.Array_Clear` _lasersattached))

(fn `ClearAttachedLasers`
  (params (ID_Clear :type String))
  (bind (_arrayindex _arrayelement) (`/Engine/EditorBlueprintResources/StandardMacros.ReverseForEachLoop` (`self.LasersAttached`))
    (:`LoopBody`
      (`/Engine/EditorBlueprintResources/StandardMacros.IsValid` _arrayelement
        (:`Is Valid`
          (if (`KismetStringLibrary.Contains` (`/Game/Interactable/Objects/Laser/BP_Laser.LaserID` _arrayelement) (`local.ID_Clear`))
            (`self.K2_DestroyActor` _arrayelement)
            (`KismetArrayLibrary.Array_RemoveItem` (`self.LasersAttached`) _arrayelement)))))))

(fn `UserConstructionScript`)