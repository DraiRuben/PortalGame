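; Laser beam segment that interacts with reflective surfaces, portals and other BPI_Lasers targets.
; Each Tick, a thin box trace along the mesh's up axis scales the beam to the impact point or maximum range.
; Hit changes notify targets or the emitter and store the returned bounce laser, while sustained hits reposition it or update the portal.
; CancelTargetHit releases or deactivates the last target, then destroys the segment unless overridden.
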(event `self.ReceiveTick`
  (params (DeltaSeconds :type "Float (single-precision)"))
  (`self.SetEndPoint`))

(fn `CancelTargetHit`
  (params (Override :type Boolean))
  (returns (`Remove From Array` :type Boolean))
  (`|ExecutionSequence`
    (:`then_0`
      (bind _lasthitactor (`self.LastHitActor`)
        (:`then`
          (bind _asbp_laser_parent (cast `/Game/Interactable/Objects/Laser/BP_LaserParent` _lasthitactor))
          (if (and (`KismetArrayLibrary.Array_IsEmpty` (`/Game/Interactable/Objects/Laser/BP_LaserParent.LasersAttached` _asbp_laser_parent)) (`KismetSystemLibrary.DoesImplementInterface` _asbp_laser_parent "/Game/Interactable/Objects/Laser/BPI_Lasers.BPI_Lasers_C"))
            (message `/Game/Interactable/Objects/Laser/BPI_Lasers.LaserBounce` (`self.LastHitActor`) self false (struct))
            (else
              (set `/Game/Interactable/Objects/Laser/BP_LaserParent.Active` false _asbp_laser_parent))))
        (:`else`)))
    (:`then_1`
      (if (`local.Override`)
        (return false)
        (else
          (`self.K2_DestroyActor`)
          (return true))))))

(fn `DifferentActorHit`
  (params (HitActor :type "Object Object Reference") (HitInfo :type "HitResult Structure"))
  (`|ExecutionSequence`
    (:`then_0`
      (if (`KismetSystemLibrary.DoesImplementInterface` (`self.LastHitActor`) "/Game/Interactable/Objects/Laser/BPI_Lasers.BPI_Lasers_C")
        (`/Game/Interactable/Objects/Laser/BP_LaserEmitter.RemoveFollowingLasers` (`self.LaserEmitter`) self)))
    (:`then_1`
      (if (`KismetSystemLibrary.DoesImplementInterface` (`local.HitActor`) "/Game/Interactable/Objects/Laser/BPI_Lasers.BPI_Lasers_C")
        (bind _newlaser (message `/Game/Interactable/Objects/Laser/BPI_Lasers.LaserBounce` HitActor self true HitInfo))
        (set `self.BounceLaser` _newlaser)))))

(fn `NothingHit`
  (params (HitInfo :type "HitResult Structure") (HitActor :type "Actor Object Reference"))
  (`|ExecutionSequence`
    (:`then_0`
      (`self.LastHitActor`
        (:`then`
          (if (`KismetSystemLibrary.DoesImplementInterface` HitActor)
            (message `/Game/Interactable/Objects/Laser/BPI_Lasers.LaserBounce` (`self.LastHitActor`) self false HitInfo)))
        (:`else`)))
    (:`then_1`
      (set `self.LastHitActor` null)
      (set `self.BounceLaser` null))))

(fn `SameActorHit`
  (params (Hit :type "HitResult Structure (by ref)"))
  (bind _lasthitactor (`self.LastHitActor`))
  (cast `/Game/Interactable/Objects/Laser/BP_ReflectiveSurface` _lasthitactor
    (:`then`
      (`self.K2_SetActorLocation` (`self.BounceLaser`) (`.ImpactPoint` (`GameplayStatics.BreakHitResult` Hit)) false false))
    (:`CastFailed`
      (bind _asbp_portal (cast `/Game/Portal/BP_Portal` _lasthitactor))
      (`/Game/Interactable/Objects/Laser/BPI_Lasers.LaserBounce` _asbp_portal self true Hit))))

(fn `SetEndPoint`
  (locals (HitActor :type "Actor Object Reference") (HitInfo :type "HitResult Structure"))
  (bind _sm_parent (`self.SM_Parent`))
  (bind (_returnvalue_x _returnvalue_y) (`KismetMathLibrary.BreakVector` (`SceneComponent.K2_GetComponentScale` (`self.SM_Parent`))))
  (bind _returnvalue (`SceneComponent.GetUpVector` _sm_parent))
  (bind _returnvalue_2 (+ (`SceneComponent.K2_GetComponentLocation` _sm_parent) (* _returnvalue 2.0)))
  (bind _outhit (`KismetSystemLibrary.BoxTraceSingle` _returnvalue_2 (+ _returnvalue_2 (* _returnvalue (`self.Range`))) (0.5 0.5 0.5) (struct) "TraceTypeQuery2" false (`self.ToIgnore`)))
  (bind _output_get (set `local.HitInfo` _outhit))
  (bind (_bblockinghit _binitialoverlap _time _distance _location _impactpoint _normal _impactnormal _physmat _hitactor) (`GameplayStatics.BreakHitResult` _output_get))
  (set `local.HitActor` _hitactor)
  (`SceneComponent.SetWorldScale3D` (`self.SM_Parent`) (`KismetMathLibrary.MakeVector` _returnvalue_x _returnvalue_y (`KismetMathLibrary.SelectFloat` (/ (+ (`KismetMathLibrary.Vector_Distance` _returnvalue_2 _impactpoint) 1.0) 200.0) (/ (`self.Range`) 200.0) _bblockinghit)))
  (`local.HitActor`
    (:`then`
      (`|ExecutionSequence`
        (:`then_0`
          (if (== (`self.LastHitActor`) (`local.HitActor`))
            (`self.SameActorHit` (`local.HitInfo`))
            (else
              (`self.DifferentActorHit` (`local.HitActor`) (`local.HitInfo`)))))
        (:`then_1`
          (set `self.LastHitActor` (`local.HitActor`)))))
    (:`else`
      (`self.NothingHit` (`local.HitInfo`) (`local.HitActor`)))))

(fn `UpdateID`
  (params (AppendValue :type String))
  (returns (NewID :type String))
  (return (`KismetStringLibrary.Concat_StrStr` (`self.LaserID`) AppendValue)))

(fn `UserConstructionScript`
  (`parent.UserConstructionScript`))