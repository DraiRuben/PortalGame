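; Reflective cube that can be picked up through BPCPickable and redirects an incoming laser along its arrow's forward direction.
; When first hit, LaserBounce spawns a child BP_Laser just ahead of the arrow, attached to the cube so it follows its movement.
; The new laser gets an updated ID and is registered with the originating emitter.
; Further hits are ignored while active, and losing the hit clears all attached lasers.
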(fn `Interact`
  (params (InteractingActor :type "Actor Object Reference"))
  (returns (HasInteracted :type Boolean))
  (bind _hasinteracted (`/Game/Interactable/BPC_Interactable.Interact` (`self.BPC_Pickable`) InteractingActor))
  (return _hasinteracted))

(fn `LaserBounce`
  (params (HitLaser :type "/Game/Interactable/Objects/Laser/BP_Laser Object Reference") (Hit :type Boolean) (HitInfo :type "HitResult Structure"))
  (returns (NewLaser :type "/Game/Interactable/Objects/Laser/BP_Laser Object Reference"))
  (bind _arrow (`self.Arrow`))
  (bind _returnvalue (`SceneComponent.GetForwardVector` _arrow))
  (`/Engine/EditorBlueprintResources/StandardMacros.IsValid` HitLaser
    (:`Is Valid`
      (set `self.LaserEmitter` (`/Game/Interactable/Objects/Laser/BP_LaserParent.LaserEmitter` HitLaser))
      (if (or (and (`local.Hit`) (not (`self.Active`))) (not (`local.Hit`)))
        (bind _output_get (set `self.Active` (`local.Hit`)))
        (if _output_get
          (bind _returnvalue_2 (`|SpawnActorFromClass` "/Game/Interactable/Objects/Laser/BP_Laser.BP_Laser_C" (`KismetMathLibrary.MakeTransform` (+ (`SceneComponent.K2_GetComponentLocation` _arrow) (* _returnvalue 65.0)) (`KismetMathLibrary.MakeRotFromX` _returnvalue)) "Undefined" "MultiplyWithRoot" null (`/Game/Interactable/Objects/Laser/BP_Laser.UpdateID` (`local.HitLaser`) "C") (`self.LaserEmitter`) null))
          (`self.K2_AttachToComponent` _returnvalue_2 (`self.SM_Parent`) "None" "KeepWorld" "KeepWorld" "KeepRelative" false)
          (`KismetArrayLibrary.Array_Add` (`self.LasersAttached`) _returnvalue_2)
          (`KismetArrayLibrary.Array_Add` (`/Game/Interactable/Objects/Laser/BP_LaserEmitter.Child Lasers` (`self.LaserEmitter`)) _returnvalue_2)
          (return _returnvalue_2)
          (else
            (`self.ClearAllAttachedLasers`)))))))

(fn `UserConstructionScript`)