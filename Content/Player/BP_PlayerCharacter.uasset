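; First-person player character with Enhanced Input movement, look, jump and hold-to-grab interaction.
; Interact line-traces for an actor, sends it InteractMessage and grabs the hit component with a physics handle, which Tick holds at its original distance along the camera's forward vector.
; Releasing input messages the actor again and drops it if the externally set IsInteracting flag is true.
; SmoothReorient uses a timeline to ease a rolled controller and capsule back upright.
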(event `self.ReceiveBeginPlay`
  (`self.K2_SetActorLocationAndRotation` (0.0 0.0 0.0)))

(event `self.ReceiveTick`
  (params (DeltaSeconds :type "Float (single-precision)"))
  (`self.UpdateGrabbedObjectPos`))

(event `EnhancedInput|/Game/Input/InputActions/IA_Move`
  (params (ActionValue :type "Vector2D Structure") (ElapsedSeconds :type "Float (double-precision)") (TriggeredSeconds :type "Float (double-precision)") (InputAction :type "InputAction Object Reference" :default "/Game/Input/InputActions/IA_Move.IA_Move"))
  (bind (_returnvalue_x _returnvalue_y) (`KismetMathLibrary.BreakVector2D` (* ActionValue (`self.Movement Speed`))))
  (:`Triggered`
    (`PawnMovementComponent.AddInputVector` (`self.CharacterMovement`) (+ (* _returnvalue_x (`self.GetActorForwardVector`)) (* _returnvalue_y (`self.GetActorRightVector`))) false)))

(event `EnhancedInput|/Game/Input/InputActions/IA_CameraMove`
  (params (ActionValue :type "Vector2D Structure") (ElapsedSeconds :type "Float (double-precision)") (TriggeredSeconds :type "Float (double-precision)") (InputAction :type "InputAction Object Reference" :default "/Game/Input/InputActions/IA_CameraMove.IA_CameraMove"))
  (bind (_returnvalue_x _returnvalue_y) (`KismetMathLibrary.BreakVector2D` (* ActionValue (`self.Sensitivity`))))
  (:`Triggered`
    (`self.AddControllerYawInput` _returnvalue_x)
    (`self.AddControllerPitchInput` (* _returnvalue_y -1.0))))

(event `/Game/Player/BPI_Player.SmoothReorient`
  (params (`New Control Rotation` :type "Rotator Structure"))
  (bind _capsulecomponent (`self.CapsuleComponent`))
  (bind _initial_control_rotation (`self.Initial Control Rotation`))
  (bind (_initial_world_rotation_roll _initial_world_rotation_pitch) (`KismetMathLibrary.BreakRotator` (`self.Initial World Rotation`)))
  (bind _returnvalue_roll (`KismetMathLibrary.BreakRotator` (`SceneComponent.K2_GetComponentRotation` (`self.CapsuleComponent`))))
  (bind (_returnvalue_roll_2 _returnvalue_pitch _returnvalue_yaw) (`KismetMathLibrary.BreakRotator` (`SceneComponent.K2_GetComponentRotation` _capsulecomponent)))
  (bind _returnvalue_roll_3 (`KismetMathLibrary.BreakRotator` (`Controller.GetControlRotation` (`GameplayStatics.GetPlayerController` 0))))
  (if (or (!= _returnvalue_roll_3 0.0) (!= _returnvalue_roll 0.0))
    (set `self.Initial Control Rotation` (`Controller.GetControlRotation` (`GameplayStatics.GetPlayerController` 0)))
    (set `self.Initial World Rotation` (`SceneComponent.K2_GetComponentRotation` (`self.CapsuleComponent`)))
    (`TimelineComponent.SetPlayRate` (`self.Rotate`) (/ 1.0 (`self.ReorientationTime`)))
    (bind (_direction _alpha) (`Timeline|Rotate` :!via `PlayFromStart`)
      (:`Update`
        (`Controller.SetControlRotation` (`GameplayStatics.GetPlayerController` 0) (`|EaseFunction` "EaseInOut" _alpha _initial_control_rotation (`KismetMathLibrary.MakeRotator` 0.0 (.pitch _initial_control_rotation) (.yaw _initial_control_rotation))))
        (`SceneComponent.K2_SetWorldRotation` _capsulecomponent (`KismetMathLibrary.MakeRotator` (`KismetMathLibrary.Lerp` _initial_world_rotation_roll 0.0 _alpha) (`KismetMathLibrary.Lerp` _initial_world_rotation_pitch 0.0 _alpha) _returnvalue_yaw) false false)))))

(event `EnhancedInput|/Game/Input/InputActions/IA_Jump`
  (params (ActionValue :type Boolean) (ElapsedSeconds :type "Float (double-precision)") (TriggeredSeconds :type "Float (double-precision)") (InputAction :type "InputAction Object Reference" :default "/Game/Input/InputActions/IA_Jump.IA_Jump"))
  (:`Started`
    (`self.Jump`)))

(event `/Game/Player/BPI_Player.SetInteracting`
  (params (Interacting :type Boolean) (InteractingActor :type "Actor Object Reference"))
  (set `self.IsInteracting` Interacting)
  (set `self.InteractingActor` InteractingActor))

(event `EnhancedInput|/Game/Input/InputActions/IA_Interact`
  (params (ActionValue :type Boolean) (ElapsedSeconds :type "Float (double-precision)") (TriggeredSeconds :type "Float (double-precision)") (InputAction :type "InputAction Object Reference" :default "/Game/Input/InputActions/IA_Interact.IA_Interact"))
  (bind (_trace_start _trace_end) (`/Game/Systems/BPFL_FunctionLibrary.Get Trace` 500.0))
  (:`Started`
    (if (not (`self.IsInteracting`))
      (bind (_outhit _returnvalue) (`KismetSystemLibrary.LineTraceSingle` :`Start` _trace_start :`End` _trace_end :`TraceChannel` "TraceTypeQuery1" :`DrawDebugType` "ForDuration"))
      (if _returnvalue
        (bind (_bblockinghit _binitialoverlap _time _distance _location _impactpoint _normal _impactnormal _physmat _hitactor _hitcomponent) (`GameplayStatics.BreakHitResult` _outhit))
        (bind _hasinteracted (message `/Game/Interactable/BPI_Interactable.Interact` _hitactor self))
        (if _hasinteracted
          (bind _returnvalue_2 (`SceneComponent.K2_GetComponentLocation` _hitcomponent))
          (set `self.LastGrabbedDist` (`KismetMathLibrary.Vector_Distance` _returnvalue_2 (`SceneComponent.K2_GetComponentLocation` (`self.Camera`))))
          (set `self.InteractingActor` _hitactor)
          (`PhysicsHandleComponent.GrabComponentAtLocationWithRotation` (`self.HandHandle`) _hitcomponent "None" _returnvalue_2 (`SceneComponent.K2_GetComponentRotation` _hitcomponent))))))
  (:`Canceled`
    (if (`self.IsInteracting`) :!label _label
      (message `/Game/Interactable/BPI_Interactable.Interact` (`self.InteractingActor`) self)
      (`PhysicsHandleComponent.ReleaseComponent` (`self.HandHandle`))))
  (:`Completed`
    (goto _label)))

(fn `UserConstructionScript`)