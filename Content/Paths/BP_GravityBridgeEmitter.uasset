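; BP_GravityBridgeEmitter is an emitter actor that creates a gravity bridge when play begins.
; On BeginPlay it spawns a BP_GravityBridge at its Arrow component's location with the actor's rotation.
; It passes itself and its display name as the bridge's LaserEmitter and LaserID, then adds the bridge to its ChildLasers array.
; Overlap and Tick events are disabled, and the construction script only calls its parent.
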(event `self.ReceiveBeginPlay`
  (set `self.LaserEmitter` self)
  (set `self.ID` (`KismetSystemLibrary.GetDisplayName` self))
  (bind _returnvalue (`|SpawnActorFromClass` :`Class` "/Game/Paths/BP_GravityBridge.BP_GravityBridge_C" :`SpawnTransform` (`KismetMathLibrary.MakeTransform` (`SceneComponent.K2_GetComponentLocation` (`self.Arrow`)) (`self.K2_GetActorRotation`)) :`CollisionHandlingOverride` "Undefined" :`TransformScaleMethod` "MultiplyWithRoot" :`LaserID` (`self.ID`) :`LaserEmitter` (`self.LaserEmitter`) :`Instigator` null))
  (`KismetArrayLibrary.Array_Add` (`self.Child Lasers`) _returnvalue))

(fn `UserConstructionScript`
  (`parent.UserConstructionScript`))