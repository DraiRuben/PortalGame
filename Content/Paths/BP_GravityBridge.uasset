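; Gravity bridge actor that suspends gravity for the player and physics bodies inside it and carries them along its up axis.
; Overlap events track bodies and the player's movement component, damp their velocity on entry and restore gravity on exit.
; Tick pulls them toward the beam's center line with a distance-curve-scaled force, using camera location for the player, and pushes along the axis below a speed cap.
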(event `self.ReceiveTick`
  (params (DeltaSeconds :type "Float (single-precision)"))
  (bind _player (`self.Player`))
  (bind _vectortocenter (`self.GetVectorToBeamCenter` (`PlayerCameraManager.GetCameraLocation` (`GameplayStatics.GetPlayerCameraManager` 0))))
  (`parent.ReceiveTick` DeltaSeconds)
  (for _array_element (`self.OverlappingBodies`)
    (`/Engine/EditorBlueprintResources/StandardMacros.IsValid` _array_element
      (:`Is Valid`
        (`PrimitiveComponent.SetPhysicsAngularVelocityInDegrees` _array_element (0.0 0.0 0.0) false "None")
        (bind _vectortocenter_2 (`self.GetVectorToBeamCenter` (`SceneComponent.K2_GetComponentLocation` _array_element)))
        (`PrimitiveComponent.AddForce` _array_element (* (* _vectortocenter_2 (`PortalsFunctionLibrary.GetRuntimeFloatCurveValue` (`self.In Curve`) (/ (`KismetMathLibrary.VSize` _vectortocenter_2) 100.0))) 5.0) "None" true)
        (if (< (`KismetMathLibrary.VSize` (`SceneComponent.GetComponentVelocity` _array_element)) 600.0)
          (`PrimitiveComponent.AddForce` _array_element (* (`SceneComponent.GetUpVector` (`self.SM_Parent`)) 400.0) "None" true)))))
  (`/Engine/EditorBlueprintResources/StandardMacros.IsValid` _player
    (:`Is Valid`
      (`CharacterMovementComponent.AddForce` _player (* (* _vectortocenter (`PortalsFunctionLibrary.GetRuntimeFloatCurveValue` (`self.In Curve`) (/ (`KismetMathLibrary.VSize` _vectortocenter) 100.0))) 5.0))
      (if (< (`KismetMathLibrary.VSize` (`MovementComponent.Velocity` _player)) 600.0)
        (`CharacterMovementComponent.AddForce` _player (* (`SceneComponent.GetUpVector` (`self.SM_Parent`)) 500.0))))))

(event `self.SM_Parent.OnComponentBeginOverlap`
  (params (OverlappedComponent :type "PrimitiveComponent Object Reference") (OtherActor :type "Actor Object Reference") (OtherComp :type "PrimitiveComponent Object Reference") (OtherBodyIndex :type Integer) (bFromSweep :type Boolean) (SweepResult :type "HitResult Structure (by ref)"))
  (`PrimitiveComponent.SetEnableGravity` OtherComp false)
  (if (`KismetSystemLibrary.DoesImplementInterface` OtherActor "/Game/Player/BPI_Player.BPI_Player_C")
    (bind _output_get (set `self.Player` (`self.GetComponentByClass` OtherActor "/Script/Engine.CharacterMovementComponent")))
    (set `CharacterMovementComponent.GravityScale` 0.0 _output_get)
    (set `MovementComponent.Velocity` (/ (`MovementComponent.Velocity` _output_get) 100.0) _output_get)
    (else
      (`KismetArrayLibrary.Array_AddUnique` (`self.OverlappingBodies`) OtherComp)
      (`PrimitiveComponent.SetPhysicsLinearVelocity` OtherComp (/ (`SceneComponent.GetComponentVelocity` OtherComp) 100.0) false "None")
      (`PrimitiveComponent.SetPhysicsAngularVelocityInDegrees` OtherComp (0.0 0.0 0.0) false "None"))))

(event `self.SM_Parent.OnComponentEndOverlap`
  (params (OverlappedComponent :type "PrimitiveComponent Object Reference") (OtherActor :type "Actor Object Reference") (OtherComp :type "PrimitiveComponent Object Reference") (OtherBodyIndex :type Integer))
  (`PrimitiveComponent.SetEnableGravity` OtherComp true)
  (`KismetArrayLibrary.Array_RemoveItem` (`self.OverlappingBodies`) OtherComp)
  (if (`KismetSystemLibrary.DoesImplementInterface` OtherActor "/Game/Player/BPI_Player.BPI_Player_C")
    (bind _player (`self.Player`)
      (:`then`
        (set `CharacterMovementComponent.GravityScale` 1.0 _player)
        (set `self.Player` null)
        (`KismetSystemLibrary.PrintString` (`KismetSystemLibrary.GetDisplayName` OtherComp)))
      (:`else`))))

(fn `GetVectorToBeamCenter`
  (params (Location :type "Vector Structure"))
  (returns (VectorToCenter :type "Vector Structure"))
  (bind _returnvalue (`SceneComponent.GetUpVector` (`self.SM_Parent`)))
  (bind _returnvalue_2 (`SceneComponent.K2_GetComponentLocation` (`self.SM_Parent`)))
  (return (- (+ (* _returnvalue (`KismetMathLibrary.Dot_VectorVector` _returnvalue (- Location _returnvalue_2))) _returnvalue_2) Location)))

(fn `UserConstructionScript`
  (`parent.UserConstructionScript`))